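; MotherRabbit_BP is the mother rabbit character Blueprint, holding unfinished experiments in jump feel.
; Two custom events set a heavier gravity scale at the jump apex and restore normal gravity on reaching the ground.
; Their delegate bindings, apex notification and a launch-based double jump sit in disconnected chains that never run.
; The jump input, BeginPlay, overlap and Tick events are all empty.
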(event `EnhancedInput|/Game/Blueprints/Characters/MotherRabbit/Input/IA_Jump`
  (params (ActionValue :type Boolean) (ElapsedSeconds :type "Float (double-precision)") (TriggeredSeconds :type "Float (double-precision)") (InputAction :type "InputAction Object Reference" :default "/Game/Blueprints/Characters/MotherRabbit/Input/IA_Jump.IA_Jump")))

(event `self.ReceiveBeginPlay`)

(event `OnReachedJumpApex_Event`
  (`KismetSystemLibrary.PrintString` "Hello")
  (set `CharacterMovementComponent.GravityScale` 2.0 (`self.CharacterMovement`)))

(event `OnReachingGround_Event`
  (set `CharacterMovementComponent.GravityScale` 1.0 (`self.CharacterMovement`)))

(event `EnhancedInput|/Game/Blueprints/Characters/MotherRabbit/Input/IA_Jump`
  (params (ActionValue :type Boolean) (ElapsedSeconds :type "Float (double-precision)") (TriggeredSeconds :type "Float (double-precision)") (InputAction :type "InputAction Object Reference" :default "/Game/Blueprints/Characters/MotherRabbit/Input/IA_Jump.IA_Jump")))

(event `self.ReceiveTick`
  (params (DeltaSeconds :type "Float (single-precision)")))

(event `self.ReceiveActorBeginOverlap`
  (params (OtherActor :type "Actor Object Reference")))

(fn `UserConstructionScript`)