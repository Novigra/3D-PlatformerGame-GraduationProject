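; TestSubject is a playground test actor that turns to face the MotherRabbit once it has overlapped it.
; The first successful overlap cast caches the rabbit in PlayerRef and prints its name; later overlaps by any actor just reprint that name.
; While the reference is valid, Tick smoothly rotates the whole actor toward the rabbit's location with RInterpTo, even after the overlap ends.
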(event `self.ReceiveActorBeginOverlap`
  (params (OtherActor :type "Actor Object Reference"))
  (`/Engine/EditorBlueprintResources/StandardMacros.IsValid` (`self.PlayerRef`)
    (:`Is Valid`
      (`KismetSystemLibrary.PrintString` (`KismetSystemLibrary.GetDisplayName` (`self.PlayerRef`))))
    (:`Is Not Valid`
      (bind _asmother_rabbit (cast `MotherRabbit` OtherActor))
      (bind _output_get (set `self.PlayerRef` _asmother_rabbit))
      (`KismetSystemLibrary.PrintString` (`KismetSystemLibrary.GetDisplayName` _output_get)))))

(event `self.ReceiveTick`
  (params (DeltaSeconds :type "Float (single-precision)"))
  (bind _playerref (`self.PlayerRef`))
  (`/Engine/EditorBlueprintResources/StandardMacros.IsValid` _playerref
    (:`Is Valid`
      (`self.K2_SetActorRotation` (`KismetMathLibrary.RInterpTo` (`self.K2_GetActorRotation`) (`KismetMathLibrary.Conv_VectorToRotator` (`KismetMathLibrary.Normal` (- (`self.K2_GetActorLocation` _playerref) (`self.K2_GetActorLocation`)))) DeltaSeconds 20.0)))))

(fn `UserConstructionScript`)